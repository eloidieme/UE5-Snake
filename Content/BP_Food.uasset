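; BP_Food is the food pickup in a Snake game, relocating and growing the snake when overlapped.
; On any actor overlap, with no check on which actor, it teleports to a random cell on a 100-unit grid centered on the origin at a fixed height.
; It then looks up BP_SnakeHead with GetActorOfClass and calls SpawnBodyElement on it to add a body segment.
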(event `self.ReceiveBeginPlay`)

(event `self.ReceiveActorBeginOverlap`
  (params (OtherActor :type "Actor Object Reference"))
  (`self.K2_SetActorLocation` (`KismetMathLibrary.MakeVector` (`KismetMathLibrary.Conv_IntToDouble` (- (* (`KismetMathLibrary.RandomIntegerInRange` 0 27) 100) 1350)) (`KismetMathLibrary.Conv_IntToDouble` (- (* (`KismetMathLibrary.RandomIntegerInRange` 0 27) 100) 1350)) 40.0))
  (bind _returnvalue (`GameplayStatics.GetActorOfClass` "/Game/BP_SnakeHead.BP_SnakeHead_C"))
  (`/Game/BP_SnakeHead.SpawnBodyElement` _returnvalue))

(fn `UserConstructionScript`)