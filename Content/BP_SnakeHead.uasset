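; BP_SnakeHead is the player-controlled snake head in a grid-based Snake game, steered by four directional inputs and spawning food at BeginPlay.
; A looping timer steps the head one cell, wrapping it at bounds with its mesh hidden, and shifts each body segment into its predecessor's previous position.
; SpawnBodyElement grows parallel segment, position and overlap-flag arrays.
; Overlapping a segment resets the game only once that segment has moved, sparing newly spawned ones.
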(event `InputAction|DownDirection`
  (params (Key :type "Key Structure"))
  ;[1 0.2224 0.7436] Handle Input
  (:`Pressed`
    (set `self.CurrentDirection` (0.0 1.0 0.0))))

(event `InputAction|UpDirection`
  (params (Key :type "Key Structure"))
  ;[1 0.2224 0.7436] Handle Input
  (:`Pressed`
    (set `self.CurrentDirection` (0.0 -1.0 0.0))))

(event `InputAction|RightDirection`
  (params (Key :type "Key Structure"))
  ;[1 0.2224 0.7436] Handle Input
  (:`Pressed`
    (set `self.CurrentDirection` (1.0 0.0 0.0))))

(event `InputAction|LeftDirection`
  (params (Key :type "Key Structure"))
  ;[1 0.2224 0.7436] Handle Input
  (:`Pressed`
    (set `self.CurrentDirection` (-1.0 0.0 0.0))))

(event `self.ReceiveBeginPlay`
  (`self.SpawnFood`)
  (`KismetSystemLibrary.K2_SetTimer` null "MoveBody" (`self.timeInterval`) true))

(event `self.ReceiveActorBeginOverlap`
  (params (OtherActor :type "Actor Object Reference"))
  (`self.HandleCollisionWithBody` OtherActor))

(fn `CheckLeftBound`
  (params (CurrentPosition :type "Vector Structure"))
  (returns (IsBeforeLeft :type Boolean))
  (return (< (.x CurrentPosition) (* (`self.boundCoord`) -1.0))))

(fn `CheckLowerBound`
  (params (CurrentPosition :type "Vector Structure"))
  (returns (isBelowLower :type Boolean))
  (return (> (.y CurrentPosition) (`self.boundCoord`))))

(fn `CheckRightBound`
  (params (CurrentPosition :type "Vector Structure"))
  (returns (IsAfterRight :type Boolean))
  (return (> (.x CurrentPosition) (`self.boundCoord`))))

(fn `CheckUpperBound`
  (params (CurrentPosition :type "Vector Structure"))
  (returns (isAboveUpper :type Boolean))
  (return (< (.y CurrentPosition) (* (`self.boundCoord`) -1.0))))

(fn `HandleCollisionWithBody`
  (params (OverlapObject :type "Object Object Reference"))
  (bind _asbp_snake_body (cast `/Game/BP_SnakeBody` OverlapObject))
  (if (`|GetArrayItem` (`self.OverlapStatus`) (`KismetArrayLibrary.Array_Find` (`self.BodySegments`) _asbp_snake_body))
    (`self.ResetGame`)))

(fn `Move Head`
  (bind _returnvalue (`self.K2_GetActorLocation`))
  (if (`self.CheckLowerBound` _returnvalue)
    (`self.WrapHead` (`self.MoveToLower` _returnvalue))
    (elif (`self.CheckUpperBound` _returnvalue)
      (`self.WrapHead` (`self.MoveToUpper` _returnvalue))
      (elif (`self.CheckRightBound` _returnvalue)
        (`self.WrapHead` (`self.MoveToLeft` _returnvalue))
        (elif (`self.CheckLeftBound` _returnvalue)
          (`self.WrapHead` (`self.MoveToRight` _returnvalue))
          (else
            (`self.K2_SetActorLocation` (`self.MoveNormal` _returnvalue) false true)))))))

(fn `MoveBody`
  (set `self.PreviousPosition` (`self.K2_GetActorLocation`))
  (`self.Move Head`)
  (for (_array_element _array_index) (`self.BodySegments`)
    (if (== _array_index 0)
      (`KismetArrayLibrary.Array_Set` (`self.PreviousPositions`) _array_index (`self.K2_GetActorLocation` _array_element))
      (`self.K2_SetActorLocation` _array_element (`self.PreviousPosition`) false false)
      (`KismetArrayLibrary.Array_Set` (`self.OverlapStatus`) _array_index true)
      (else
        (`self.MoveBodyElement` _array_element _array_index)))))

(fn `MoveBodyElement`
  (params (BodyElement :type "/Game/BP_SnakeBody Object Reference") (ElementIndex :type Integer))
  (bind _previouspositions (`self.PreviousPositions`))
  (`KismetArrayLibrary.Array_Set` _previouspositions ElementIndex (`self.K2_GetActorLocation` BodyElement))
  (`self.K2_SetActorLocation` BodyElement (`|GetArrayItem` _previouspositions (- ElementIndex 1)) false false)
  (`KismetArrayLibrary.Array_Set` (`self.OverlapStatus`) ElementIndex true))

(fn `MoveNormal`
  (params (currentPosition :type "Vector Structure"))
  (returns (NewPosition :type "Vector Structure"))
  (return (+ (* (`self.CurrentDirection`) (`self.cellSize`)) currentPosition)))

(fn `MoveToLeft`
  (params (currentPosition :type "Vector Structure"))
  (returns (newPosition :type "Vector Structure"))
  (return (`KismetMathLibrary.MakeVector` (* (`self.boundCoord`) -1.0) (.y currentPosition) (.z currentPosition))))

(fn `MoveToLower`
  (params (currentPosition :type "Vector Structure"))
  (returns (newPosition :type "Vector Structure"))
  (return (`KismetMathLibrary.MakeVector` (.x currentPosition) (* (`self.boundCoord`) -1.0) (.z currentPosition))))

(fn `MoveToRight`
  (params (currentPosition :type "Vector Structure"))
  (returns (newPosition :type "Vector Structure"))
  (return (`KismetMathLibrary.MakeVector` (`self.boundCoord`) (.y currentPosition) (.z currentPosition))))

(fn `MoveToUpper`
  (params (CurrentPosition :type "Vector Structure"))
  (returns (NewPosition :type "Vector Structure"))
  (return (`KismetMathLibrary.MakeVector` (.x CurrentPosition) (`self.boundCoord`) (.z CurrentPosition))))

(fn `ResetGame`
  (bind _bodysegments (`self.BodySegments`))
  (for _array_element _bodysegments
    (`self.K2_DestroyActor` _array_element))
  (`KismetArrayLibrary.Array_Clear` _bodysegments)
  (`KismetArrayLibrary.Array_Clear` (`self.PreviousPositions`))
  (`KismetArrayLibrary.Array_Clear` (`self.OverlapStatus`))
  (set `self.CurrentDirection` (0.0 0.0 0.0))
  (`self.K2_SetActorLocation` (-50.0 50.0 40.0) false true))

(fn `SpawnBodyElement`
  (bind _returnvalue (- (`self.K2_GetActorLocation`) (`self.CurrentDirection`)))
  (bind _returnvalue_2 (`|SpawnActorFromClass` "/Game/BP_SnakeBody.BP_SnakeBody_C" (`KismetMathLibrary.MakeTransform` _returnvalue (.rotation (`self.GetTransform`)) (.scale (`self.GetTransform`))) "Undefined" "OverrideRootScale" null null))
  (`KismetArrayLibrary.Array_Add` (`self.BodySegments`) _returnvalue_2)
  (`KismetArrayLibrary.Array_Add` (`self.PreviousPositions`) _returnvalue)
  (`KismetArrayLibrary.Array_Add` (`self.OverlapStatus`)))

(fn `SpawnFood`
  (`|SpawnActorFromClass` "/Game/BP_Food.BP_Food_C" (`KismetMathLibrary.MakeTransform` (`KismetMathLibrary.MakeVector` (`KismetMathLibrary.Conv_IntToDouble` (- (* (`KismetMathLibrary.RandomIntegerInRange` 0 27) 100) 1350)) (`KismetMathLibrary.Conv_IntToDouble` (- (* (`KismetMathLibrary.RandomIntegerInRange` 0 27) 100) 1350)) 40.0)) "Undefined" "OverrideRootScale" null null))

(fn `UserConstructionScript`)

(fn `WrapHead`
  (params (NewLocation :type "Vector Structure"))
  (`SceneComponent.SetVisibility` (`self.Cube`) false false)
  (`self.K2_SetActorLocation` NewLocation false true)
  (`SceneComponent.SetVisibility` (`self.Cube`) true false))